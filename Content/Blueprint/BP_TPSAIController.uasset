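; AI controller for third-person shooter characters that turns perception events into blackboard state for enemy detection.
; On perception updates, it takes the first updated character outside the pawn's Teammates, stores its location in the EnemyActor vector key, stops movement and sets SeeEnemy.
; When any perceived target is forgotten, it clears SeeEnemy but leaves the stored location.
; Both handlers print debug text.
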(event `self.AIPerception.OnPerceptionUpdated`
  (params (UpdatedActors :type "Array of Actor Object Reference (by ref)"))
  (bind _returnvalue (`self.K2_GetPawn`))
  (bind _enemyactor (`self.EnemyActor`))
  (bind _seeenemy (`self.SeeEnemy`))
  (bind _returnvalue_2 (`AIBlueprintHelperLibrary.GetBlackboard` _returnvalue))
  (bind _info (`AIPerceptionComponent.GetActorsPerception` (`self.AIPerception`) null))
  (if (not (and (`KismetArrayLibrary.Array_IsEmpty` UpdatedActors) (not false) (`KismetArrayLibrary.Array_IsNotEmpty` (`.LastSensedStimuli` (break `ActorPerceptionBlueprintInfo` _info)))))
    (bind _astp3shoot_character (cast `TP3ShootCharacter` _returnvalue))
    (for _array_element UpdatedActors
      (bind _astp3shoot_character_2 (cast `TP3ShootCharacter` _array_element))
      (if (not (`KismetArrayLibrary.Array_Contains` (`TP3ShootCharacter.Teammates` _astp3shoot_character) _astp3shoot_character_2))
        (`BlackboardComponent.SetValueAsVector` _returnvalue_2 _enemyactor (`self.K2_GetActorLocation` _astp3shoot_character_2))
        (`self.StopMovement`)
        (`BlackboardComponent.SetValueAsBool` _returnvalue_2 _seeenemy true)
        (`KismetSystemLibrary.PrintText` (`KismetTextLibrary.Conv_StringToText` (`KismetStringLibrary.Concat_StrStr` "L'" (`KismetStringLibrary.Conv_NameToString` _enemyactor) (`KismetSystemLibrary.GetDisplayName` _astp3shoot_character_2) (`KismetStringLibrary.Conv_NameToString` _seeenemy) "true")))
        (break)))))

(event `self.AIPerception.OnTargetPerceptionForgotten`
  (params (Actor :type "Actor Object Reference"))
  (`BlackboardComponent.SetValueAsBool` (`AIBlueprintHelperLibrary.GetBlackboard` (`self.K2_GetPawn`)) (`self.SeeEnemy`) false)
  (`KismetSystemLibrary.PrintText` (`KismetTextLibrary.Conv_StringToText` (`KismetStringLibrary.Concat_StrStr` "HE FORGOR" (`KismetSystemLibrary.GetDisplayName` Actor)))))

(fn `UserConstructionScript`)